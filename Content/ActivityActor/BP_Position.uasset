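; BP_Position is a character slot under a BP_VisitMain parent actor, offering click actions to wait, perform or exit.
; WaitPossess fake-possesses the waiting character, gates Perform and Exit to that occupant, and detaches the pawn on unpossess.
; Perform triggers the parent's performance, while PerfromPossess events bind the character to the parent or notify it on release.
; Wait and Perform check the parent's state name, though CanWait compares against a misspelled "Perfromance".
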(event OnUnPossess(PerfromPossess)
  (params (PC :type My%20Player%20Controller%20Object%20Reference))
  (bind _asbp_visit_main (Utilities|Casting|CastToBP_VisitMain (Actor|GetParentActor)))
  (Default|OnShowUnpossess _asbp_visit_main)
  (Utilities|Casting|CastToMyCharacter (Pawn|GetControlledPawn PC)))

(event OnUnPossess(WaitPossess)
  (params (PC :type My%20Player%20Controller%20Object%20Reference))
  (bind _returnvalue (Pawn|GetControlledPawn PC))
  (Transformation|DetachFromActor _returnvalue "KeepWorld" "KeepWorld" "KeepWorld")
  (Utilities|Casting|CastToMyCharacter _returnvalue))

(event OnPossess(WaitPossess)
  (params (PC :type My%20Player%20Controller%20Object%20Reference))
  (Utilities|Casting|CastToMyCharacter (Pawn|GetControlledPawn PC)))

(event OnPossess(PerfromPossess)
  (params (PC :type My%20Player%20Controller%20Object%20Reference))
  (bind _asmy_character (Utilities|Casting|CastToMyCharacter (Pawn|GetControlledPawn PC)))
  (bind _asbp_visit_main (Utilities|Casting|CastToBP_VisitMain (Actor|GetParentActor)))
  (Default|BindCharacter _asbp_visit_main _asmy_character))

(event EventBeginPlay)

(event Collision|EventActorBeginOverlap
  (params (OtherActor :type Actor%20Object%20Reference)))

(event EventTick
  (params (DeltaSeconds :type Float%20%28single-precision%29)))

(event Custom|Normal_Entry)

(event Custom|Normal_Exit)

(fn ConstructionScript)

(fn CanWait
  (params (Click_Param :type Click%20Param%20Structure))
  (bind _asmy_character (Utilities|Casting|CastToMyCharacter (Pawn|GetControlledPawn (.playercontroller Click_Param))))
  (bind _returnvalue (Class|FakePossessComponent|CanbePossess (Variables|Default|GetWaitPossess) _asmy_character))
  (bind _asbp_visit_main (Utilities|Casting|CastToBP_VisitMain (Actor|GetParentActor)))
  (bind _returnvalue_2 (Class|MyActivityActor|GetCurrentStateName _asbp_visit_main))
  (return (and _returnvalue (!= _returnvalue_2 "Perfromance"))))

(fn ExecuteWait
  (params (Click_Param :type Click%20Param%20Structure))
  (Class|FakePossessComponent|FakePossess (Variables|Default|GetWaitPossess) (.playercontroller Click_Param)))

(fn CanPerform
  (params (Click_Param :type Click%20Param%20Structure))
  (bind _asmy_activity_actor (Utilities|Casting|CastToMyActivityActor (Actor|GetParentActor)))
  (bind _returnvalue (Class|MyActivityActor|GetCurrentStateName _asmy_activity_actor))
  (bind _returnvalue_2 (Class|FakePossessComponent|GetCurrentPossesser (Variables|Default|GetWaitPossess)))
  (return (and (!= _returnvalue "Performance") (== _returnvalue_2 (Pawn|GetControlledPawn (.playercontroller Click_Param))))))

(fn ExecutePerform
  (params (Click_Param :type Click%20Param%20Structure))
  (bind _asbp_visit_main (Utilities|Casting|CastToBP_VisitMain (Actor|GetParentActor)))
  (Default|OnTriggerPerformance _asbp_visit_main)
  (return))

(fn CanExit
  (params (Click_Param :type Click%20Param%20Structure))
  (bind _returnvalue (Class|FakePossessComponent|GetCurrentPossesser (Variables|Default|GetWaitPossess)))
  (return (== _returnvalue (Pawn|GetControlledPawn (.playercontroller Click_Param)))))

(fn ExecuteExit
  (params (Click_Param :type Click%20Param%20Structure))
  (Class|FakePossessComponent|FakeUnPossess (Variables|Default|GetWaitPossess) "Finished")
  (return))