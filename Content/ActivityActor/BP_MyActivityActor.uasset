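; Activity actor that toggles between Cube and Sphere states, each showing its mesh and hiding the other.
; ShowSphere fake-possesses the actor and registers the player's pawn for custom net relevancy; ShowCube reverses both.
; Possess events apply or remove a persistent effect on the third-person character, add or remove its sequence binding, and print debug text.
; Check functions gate on mesh visibility, with the Sphere check also requiring that possession is allowed.
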(event OnPossess(FakePossess)
  (params (PC :type My%20Player%20Controller%20Object%20Reference))
  (Development|PrintString "Possess" true true "(R=0.000000,G=0.660000,B=1.000000,A=1.000000)" 1e+04)
  (bind _asbp_third_person_character (Utilities|Casting|CastToBP_ThirdPersonCharacter (Pawn|GetControlledPawn PC)))
  (bind _returnvalue (Class|PersistBaseComponent|CreatePersistEffectDatabyClass (Variables|/Script/MyProject.MyCharacter|GetPersistComponent _asbp_third_person_character) "/Game/ActivityActor/MyEffectWithState.MyEffectWithState_C"))
  (Class|PersistBaseComponent|ApplyPersistEffectData (Variables|/Script/MyProject.MyCharacter|GetPersistComponent _asbp_third_person_character) _returnvalue -1.0)
  (Class|MyActivityActor|AddBinding (|GetSequenceBinding) _asbp_third_person_character))

(event OnUnPossesswithReason(FakePossess)
  (params (PC :type My%20Player%20Controller%20Object%20Reference) (Reason :type EUnPossessReason%20Enum :default "None"))
  (Development|PrintString (Utilities|String|EnumtoString Reason) true true "(R=0.000000,G=0.660000,B=1.000000,A=1.000000)" 1e+05)
  (bind _asbp_third_person_character (Utilities|Casting|CastToBP_ThirdPersonCharacter (Pawn|GetControlledPawn PC)))
  (Class|PersistBaseComponent|UnApplyPersistEffectData (Variables|/Script/MyProject.MyCharacter|GetPersistComponent (stale OnPossess(FakePossess) _asbp_third_person_character)) (stale OnPossess(FakePossess) _returnvalue))
  (Class|MyActivityActor|RemoveBinding (|GetSequenceBinding) _asbp_third_person_character))

(event Custom|Cube_Entry
  (Development|SetHiddeninGame (Variables|Default|GetCube) false false)
  (Development|SetHiddeninGame (Variables|Default|GetSphere) true false))

(event Custom|Cube_Exit)

(event Custom|Sphere_Entry
  (Development|SetHiddeninGame (Variables|Default|GetSphere) false false)
  (Development|SetHiddeninGame (Variables|Default|GetCube) true false))

(event Custom|Sphere_Exit)

(fn ConstructionScript)

(fn CheckSphereHidden
  (params (NewParam :type Click%20Param%20Structure))
  (bind _asmy_character (Utilities|Casting|CastToMyCharacter (Pawn|GetControlledPawn (.playercontroller NewParam))))
  (bind _returnvalue (Class|FakePossessComponent|CanbePossess (Variables|Default|GetFakePossess) _asmy_character))
  (return (and _returnvalue (Variables|/Script/Engine.SceneComponent|GetbHiddenInGame (Variables|Default|GetSphere)))))

(fn CheckCubeHidden
  (params (NewParam :type Click%20Param%20Structure))
  (return (Variables|/Script/Engine.SceneComponent|GetbHiddenInGame (Variables|Default|GetCube))))

(fn ShowSphere
  (params (NewParam :type Click%20Param%20Structure))
  (bind _returnvalue (Pawn|GetControlledPawn (.playercontroller NewParam)))
  (bind _netrelevantcomponent (Variables|Default|GetNetRelevantComponent))
  (Class|MyActivityActor|JumptoState "Sphere" 0.0 false)
  (Class|FakePossessComponent|FakePossess (Variables|Default|GetFakePossess) (.playercontroller NewParam))
  (bind _asmy_character (Utilities|Casting|CastToMyCharacter _returnvalue))
  (Class|MyCharacter|AddCustomNetRelevantInterface _asmy_character _netrelevantcomponent)
  (Class|CustomNetRelevantComponent|AddRelevantPawn _netrelevantcomponent _returnvalue)
  (return))

(fn ShowCube
  (params (NewParam :type Click%20Param%20Structure))
  (bind _returnvalue (Pawn|GetControlledPawn (.playercontroller NewParam)))
  (bind _netrelevantcomponent (Variables|Default|GetNetRelevantComponent))
  (Class|MyActivityActor|JumptoState "Cube" 0.0 false)
  (Class|FakePossessComponent|FakeUnPossess (Variables|Default|GetFakePossess) "Finished")
  (bind _asmy_character (Utilities|Casting|CastToMyCharacter _returnvalue))
  (Class|MyCharacter|RemoveCustomNetRelevantInterface _asmy_character _netrelevantcomponent)
  (Class|CustomNetRelevantComponent|RemoveRelevantPawn _netrelevantcomponent _returnvalue)
  (return))