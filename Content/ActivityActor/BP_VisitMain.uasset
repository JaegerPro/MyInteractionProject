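; BP_VisitMain is an activity actor that seats characters at BP_Position slots and plays a sequenced group performance with them.
; At BeginPlay it collects positions from child actor selectors; waiting players attach to the first available slot.
; Triggering switches to the Performance state, moving occupants from wait to perform fake-possession and binding them into the loaded sequence by slot index.
; Sequence end returns to Normal, releasing performers and their bindings.
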(event EventBeginPlay
  (Utilities|FlowControl|Delay 0.2)
  (for _array_element (Variables|Default|GetPositionSelectorList)
    (bind _outcomponent (Class|ComponentSelectorStatics|GetComponentbySelector self _array_element))
    (bind _as子actor组件 (Utilities|Casting|CastToChildActorComponent _outcomponent))
    (bind _asbp_position (Utilities|Casting|CastToBP_Position (Variables|/Script/Engine.ChildActorComponent|GetChildActor _as子actor组件)))
    (Utilities|Array|AddUnique (Variables|Default|GetPositionList) _asbp_position)))

(event Collision|EventActorBeginOverlap
  (params (OtherActor :type Actor%20Object%20Reference)))

(event EventTick
  (params (DeltaSeconds :type Float%20%28single-precision%29))
  (bind _returnvalue (Class|MyActivityActor|GetCurrentStateName))
  (if (== _returnvalue "Performance")
    (bind _returnvalue_2 (Class|MyActivityActor|GetCurrentSequenceIsEnd))
    (if _returnvalue_2
      (Class|MyActivityActor|JumptoState "Normal" 0.0 false))))

(event EventOnSequenceLoaded
  (for _array_element (Variables|Default|GetPositionList)
    (bind _returnvalue (Class|FakePossessComponent|GetCurrentPossesser (Variables|/Game/ActivityActor/BP_Position.BP_Position_C|GetPerfromPossess _array_element)))
    (CallFunction|BindCharacter _returnvalue)))

(event Custom|Normal_Entry)

(event Custom|Normal_Exit)

(event Custom|Performance_Entry)

(event Custom|Performance_Exit
  (for (_array_element _array_index) (Variables|Default|GetPositionList)
    (bind _returnvalue (Class|FakePossessComponent|GetCurrentPossesser (Variables|/Game/ActivityActor/BP_Position.BP_Position_C|GetPerfromPossess _array_element)))
    (Utilities|IsValid _returnvalue
      (:Is%20Valid
        (Class|FakePossessComponent|FakeUnPossess (Variables|/Game/ActivityActor/BP_Position.BP_Position_C|GetPerfromPossess _array_element) "Finished")
        (Class|MyActivityActor|RemoveBinding (|GetSequenceBinding) _returnvalue)
        (Class|MyActivityActor|RemoveBinding (|GetSequenceBinding) _returnvalue)))))

(fn ConstructionScript)

(fn CanWait
  (params (Click_Param :type Click%20Param%20Structure))
  (for _array_element (Variables|Default|GetPositionList)
    (if (Default|CanWait _array_element Click_Param)
      (return true))))

(fn ExecuteWait
  (params (Click_Param :type Click%20Param%20Structure))
  (bind _array_element (Utilities|Array|ForEachLoopwithBreak (Variables|Default|GetPositionList) :!label _label)
    (:LoopBody
      (if (Default|CanWait _array_element Click_Param)
        (Default|ExecuteWait _array_element Click_Param)
        (Transformation|AttachActorToActor (Pawn|GetControlledPawn (.PlayerController (Utilities|Struct|BreakClick_Param Click_Param))) _array_element "None" "SnapToTarget" "SnapToTarget" "SnapToTarget" true)
        (goto _label Break)))))

(fn AddorRemoveBinding
  (params (Actor :type Actor%20Object%20Reference) (Index :type Integer) (bBind :type Boolean))
  (bind _returnvalue (|GetSequenceBinding))
  (bind _returnvalue_2 (|GetSequenceBinding))
  (bind _returnvalue_3 (Utilities|Select :Index Index :Option%200 _returnvalue_2 :Option%201 _returnvalue))
  (if bBind
    (Class|MyActivityActor|AddBinding _returnvalue_3 Actor)
    (else
      (Class|MyActivityActor|RemoveBinding _returnvalue_3 Actor))))

(fn OnTriggerPerformance
  (Class|MyActivityActor|JumptoState "Performance" 0.0 false)
  (for _array_element (Variables|Default|GetPositionList)
    (bind _returnvalue (Class|FakePossessComponent|GetCurrentPossesser (Variables|/Game/ActivityActor/BP_Position.BP_Position_C|GetWaitPossess _array_element)))
    (Utilities|IsValid _returnvalue
      (:Is%20Valid
        (Class|FakePossessComponent|FakeUnPossess (Variables|/Game/ActivityActor/BP_Position.BP_Position_C|GetWaitPossess _array_element) "Finished")
        (Class|FakePossessComponent|FakePossess (Variables|/Game/ActivityActor/BP_Position.BP_Position_C|GetPerfromPossess _array_element) (Pawn|GetController _returnvalue))))))

(fn OnShowUnpossess
  (for _array_element (Variables|Default|GetPositionList)
    (bind _returnvalue (Class|FakePossessComponent|GetCurrentPossesser (Variables|/Game/ActivityActor/BP_Position.BP_Position_C|GetPerfromPossess _array_element)))
    (Utilities|IsValid _returnvalue
      (:Is%20Valid
        (Class|FakePossessComponent|FakeUnPossess (Variables|/Game/ActivityActor/BP_Position.BP_Position_C|GetPerfromPossess _array_element) "Finished")
        (Class|MyActivityActor|JumptoState "Normal" 0.0 false)))))

(fn BindCharacter
  (params (Character :type Character%20Object%20Reference))
  (for (_array_element _array_index) (Variables|Default|GetPositionList)
    (bind _returnvalue (Class|FakePossessComponent|GetCurrentPossesser (Variables|/Game/ActivityActor/BP_Position.BP_Position_C|GetPerfromPossess _array_element)))
    (if (== _returnvalue Character)
      (if (== _array_index 0)
        (Class|MyActivityActor|AddBinding (|GetSequenceBinding) _returnvalue)
        (else
          (Class|MyActivityActor|AddBinding (|GetSequenceBinding) _returnvalue))))))